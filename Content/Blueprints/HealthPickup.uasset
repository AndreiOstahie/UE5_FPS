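; Health pickup that restores a BP_FirstPersonCharacter to full health on overlap.
; Tick spins the Sphere component around its yaw axis at a constant, frame-rate-independent speed.
; The Sphere's overlap event refills Health only when it is below MaxHealth, so the pickup remains for characters already at full health.
; On use, it destroys only the Sphere component, leaving the actor itself in the level.
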(event OnComponentBeginOverlap(Sphere)
  (params (OverlappedComponent :type Primitive%20Component%20Object%20Reference) (OtherActor :type Actor%20Object%20Reference) (OtherComp :type Primitive%20Component%20Object%20Reference) (OtherBodyIndex :type Integer) (bFromSweep :type Boolean) (SweepResult :type Hit%20Result%20Structure%20%28by%20ref%29))
  (bind _asbp_first_person_character (Utilities|Casting|CastToBP_FirstPersonCharacter OtherActor))
  (if (< (Variables|/Game/FirstPerson/Blueprints/BP_FirstPersonCharacter.BP_FirstPersonCharacter_C|GetHealth _asbp_first_person_character) (Variables|/Game/FirstPerson/Blueprints/BP_FirstPersonCharacter.BP_FirstPersonCharacter_C|GetMaxHealth _asbp_first_person_character))
    (Variables|/Game/FirstPerson/Blueprints/BP_FirstPersonCharacter.BP_FirstPersonCharacter_C|SetHealth _asbp_first_person_character (Variables|/Game/FirstPerson/Blueprints/BP_FirstPersonCharacter.BP_FirstPersonCharacter_C|GetMaxHealth _asbp_first_person_character))
    (Components|DestroyComponent (Variables|Default|GetSphere))))

(event EventTick
  (params (DeltaSeconds :type Float%20%28single-precision%29))
  (bind _sphere (Variables|Default|GetSphere))
  (Utilities|IsValid _sphere
    (:Is%20Valid
      (Transformation|SetWorldRotation _sphere (Math|Rotator|MakeRotator 0.0 0.0 (+ (.yaw (Transformation|GetWorldRotation _sphere)) (* DeltaSeconds 5e+01))) false false))))

(fn ConstructionScript)